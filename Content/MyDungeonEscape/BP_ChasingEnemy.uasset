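; BP_ChasingEnemy is an enemy that continuously chases the player and ends the game when it catches them.
; From BeginPlay it runs an AI MoveTo toward player character 0, re-issuing the move after a short delay on both success and failure.
; When BP_Player overlaps its CatchRadius component, it shows the WBP_GameOver widget, switches to UI-only input with a visible cursor and pauses the game.
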(event `self.ReceiveBeginPlay`
  (`self.ChasePlayer`))

(event `ChasePlayer`
  (`|AIMoveTo` self (0.0 0.0 0.0) (`GameplayStatics.GetPlayerCharacter` 0) 100.0 true
    (:`OnSuccess`
      (`KismetSystemLibrary.Delay` 0.2)
      (`self.ChasePlayer`))
    (:`OnFail`
      (`KismetSystemLibrary.Delay` 0.2)
      (`self.ChasePlayer`))))

(event `self.CatchRadius.OnComponentBeginOverlap`
  (params (OverlappedComponent :type "PrimitiveComponent Object Reference") (OtherActor :type "Actor Object Reference") (OtherComp :type "PrimitiveComponent Object Reference") (OtherBodyIndex :type Integer) (bFromSweep :type Boolean) (SweepResult :type "HitResult Structure (by ref)"))
  (bind _returnvalue (`GameplayStatics.GetPlayerController` 0))
  (cast `/Game/MyDungeonEscape/BP_Player` OtherActor)
  (bind _returnvalue_2 (`|CreateWidget` "/Game/MyDungeonEscape/WBP_GameOver.WBP_GameOver_C" _returnvalue))
  (`UserWidget.AddToViewport` _returnvalue_2 0)
  (`WidgetBlueprintLibrary.SetInputMode_UIOnlyEx` _returnvalue _returnvalue_2)
  (set `PlayerController.bShowMouseCursor` true _returnvalue)
  (`GameplayStatics.SetGamePaused` true))

(fn `UserConstructionScript`)